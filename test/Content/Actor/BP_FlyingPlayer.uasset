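; BP_FlyingPlayer is a flying player actor that currently implements only banked turning from player input.
; The InputAxisTurn axis, scaled by TurnRate and world delta time, rolls the Boby component locally and yaws the whole actor in world space by the same amount.
; BeginPlay, overlap and Tick do nothing, and a TurnMove assignment is left unconnected.
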(event `InputAxis|InputAxisTurn`
  (params (AxisValue :type "Float (single-precision)"))
  (bind _returnvalue (* (`self.TurnRate`) (`GameplayStatics.GetWorldDeltaSeconds`) AxisValue))
  (`SceneComponent.K2_AddLocalRotation` (`self.Boby`) (`KismetMathLibrary.MakeRotator` _returnvalue) false false)
  (`self.K2_AddActorWorldRotation` (`KismetMathLibrary.MakeRotator` 0.0 0.0 _returnvalue)))

(fn `UserConstructionScript`
  (`parent.UserConstructionScript`))
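; BP_ActorPlayer is an actor that moves itself continuously forward along its own facing direction.
; Each Tick offsets its location by the forward vector scaled by MoveSpeed and delta seconds, without sweep or teleport, and accumulates elapsed time in Time.
; No input or rotation logic is connected; TurnMove appears only in unused nodes, and the construction script is empty.
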(event `Key|W`
  (params (Key :type "Key Structure")))

(event `self.ReceiveTick`
  (params (DeltaSeconds :type "Float (single-precision)"))
  (`self.K2_SetActorLocation` (+ (* (`self.GetActorForwardVector`) (* (`self.MoveSpeed`) DeltaSeconds)) (`self.K2_GetActorLocation`)))
  (set `self.Time` (+ (`self.Time`) DeltaSeconds)))

(fn `UserConstructionScript`)
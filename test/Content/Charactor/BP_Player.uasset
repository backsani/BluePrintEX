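; BP_Player is the player character Blueprint, handling basic movement, look and jump input.
; Forward and right axes feed AddMovementInput along the actor's own vectors, with the direction scaled by MoveSpeed and frame delta time.
; Turn and Lookup axes drive controller yaw and pitch through a shared TurnRate, also scaled by delta time.
; Pressing Jump calls the Character jump, with no release handling.
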(event `InputAxis|MoveForward`
  (params (AxisValue :type "Float (single-precision)"))
  (`self.AddMovementInput` (* (`self.GetActorForwardVector`) (`self.MoveSpeed`) (`GameplayStatics.GetWorldDeltaSeconds`)) AxisValue))

(event `InputAxis|Turn`
  (params (AxisValue :type "Float (single-precision)"))
  (`self.AddControllerYawInput` (* (`self.TurnRate`) (`GameplayStatics.GetWorldDeltaSeconds`) AxisValue)))

(event `InputAxis|MoveRight`
  (params (AxisValue :type "Float (single-precision)"))
  (`self.AddMovementInput` (* (`self.GetActorRightVector`) (`self.MoveSpeed`) (`GameplayStatics.GetWorldDeltaSeconds`)) AxisValue))

(event `InputAxis|Lookup`
  (params (AxisValue :type "Float (single-precision)"))
  (`self.AddControllerPitchInput` (* (`self.TurnRate`) (`GameplayStatics.GetWorldDeltaSeconds`) AxisValue)))

(event `InputAction|Jump`
  (params (Key :type "Key Structure"))
  (:`Pressed`
    (`self.Jump`)))

(fn `UserConstructionScript`)